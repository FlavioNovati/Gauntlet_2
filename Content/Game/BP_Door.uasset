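; BP_Door is a door that swings open and closed in response to switch ON and OFF events.
; Each event plays its own timeline, lerping the DoorPivot relative rotation between zero and PivotONAngle in opposite directions.
; Both timelines trigger a radial world camera shake at the door's location on every update, so the shake is re-triggered throughout the motion.
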(event EventBeginPlay)

(event Collision|EventActorBeginOverlap
  (params (OtherActor :type Actor%20Object%20Reference)))

(event EventTick
  (params (DeltaSeconds :type Float%20%28single-precision%29)))

(event EventOnSwitchON
  ;[0.15 0.15 0.15 0.5] Open Door
  (bind _alpha (Timeline|Timeline Play)
    (:Update
      (Transformation|SetRelativeRotation (Variables|Default|GetDoorPivot) (Math|Rotator|MakeRotator (.X (Math|Vector|BreakVector (Math|Vector|Lerp(Vector) "0, 0, 0" (Variables|Default|GetPivotONAngle) _alpha))) (.Y (Math|Vector|BreakVector (Math|Vector|Lerp(Vector) "0, 0, 0" (Variables|Default|GetPivotONAngle) _alpha))) (.Z (Math|Vector|BreakVector (Math|Vector|Lerp(Vector) "0, 0, 0" (Variables|Default|GetPivotONAngle) _alpha)))) false false)
      (Camera|PlayWorldCameraShake "/Game/Game/Effects/CameraShake/BP_CameraShake_DoorOpening.BP_CameraShake_DoorOpening_C" (Transformation|GetActorLocation) (Variables|Default|GetShake%20Camera%20Inner%20Radious) (Variables|Default|GetShake%20Camera%20Outer%20Radious)))))

(event EventOnSwitchOFF
  ;[0.15 0.15 0.15 0.5] Close Door
  (bind _alpha (Timeline|Timeline_0 Play)
    (:Update
      (Transformation|SetRelativeRotation (Variables|Default|GetDoorPivot) (Math|Rotator|MakeRotator (.X (Math|Vector|BreakVector (Math|Vector|Lerp(Vector) (Variables|Default|GetPivotONAngle) "0, 0, 0" _alpha))) (.Y (Math|Vector|BreakVector (Math|Vector|Lerp(Vector) (Variables|Default|GetPivotONAngle) "0, 0, 0" _alpha))) (.Z (Math|Vector|BreakVector (Math|Vector|Lerp(Vector) (Variables|Default|GetPivotONAngle) "0, 0, 0" _alpha)))) false false)
      (Camera|PlayWorldCameraShake "/Game/Game/Effects/CameraShake/BP_CameraShake_DoorOpening.BP_CameraShake_DoorOpening_C" (Transformation|GetActorLocation) (Variables|Default|GetShake%20Camera%20Inner%20Radious) (Variables|Default|GetShake%20Camera%20Outer%20Radious)))))

(fn ConstructionScript)