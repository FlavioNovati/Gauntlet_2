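; Player controller that creates the game HUD and switches between main menu, gameplay and pause states.
; On BeginPlay it adds WBP_GameHUD in its first state and binds the pause screen's main menu button and the main menu's play button.
; State events set the HUD state and pause or unpause the game.
; BeginPlay also sets overall scalability, which the author notes belongs in the Game Instance.
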(event EventBeginPlay
  ;[0 0 0 0.5] Setup
  (Utilities|FlowControl|Sequence
    (:then_0
      ;[0.15 0.15 0.15 0.5] HUD Setup
      (bind _returnvalue (UserInterface|CreateWidget "/Game/Game/HUD/WBP_GameHUD.WBP_GameHUD_C"))
      (bind _output_get (Variables|Default|SetGame%20Widget _returnvalue))
      (UserInterface|Viewport|AddtoViewport _output_get 0)
      (Default|SetHUDState (Variables|Default|GetGame%20Widget) "NewEnumerator0")
      (Utilities|FlowControl|Sequence
        (:then_0
          (bind _wbp_pausehud (Default|GetPauseHUD (Variables|Default|GetGame%20Widget)))
          (bind _main_menu_btn (Default|GetMainMenuButton _wbp_pausehud))
          (EventDispatchers|BindEventtoOnButtonPressed _main_menu_btn (EventDispatchers|CreateEvent :!event ReturntoMainMenu)))
        (:then_1
          (bind _wbp_mainmenuhud (Default|GetMainMenuHUD (Variables|Default|GetGame%20Widget)))
          (bind _play_btn (Default|GetPlayButton _wbp_mainmenuhud))
          (EventDispatchers|BindEventtoOnButtonPressed _play_btn (EventDispatchers|CreateEvent :!event Play)))))
    (:then_1
      ;[0.15 0.15 0.15 0.5] Set Up Resolution (not optimal, should be in Game Instance)
      (bind _returnvalue_2 (Settings|GetGameUserSettings))
      (Class|GameUserSettings|SetOverallScalabilityLevel _returnvalue_2 1))))

(event EventOnPause
  ;[0 0 0 0.5] Game States
  (Default|SetHUDState (Variables|Default|GetGame%20Widget) "NewEnumerator2")
  (Game|SetGamePaused true))

(event EventOnMainMenu
  ;[0 0 0 0.5] Game States
  (Default|SetHUDState (Variables|Default|GetGame%20Widget) "NewEnumerator0")
  (Game|SetGamePaused true))

(event EventOnGameplay
  ;[0 0 0 0.5] Game States
  (Default|SetHUDState (Variables|Default|GetGame%20Widget) "NewEnumerator1")
  (Game|SetGamePaused false))

(fn ConstructionScript)