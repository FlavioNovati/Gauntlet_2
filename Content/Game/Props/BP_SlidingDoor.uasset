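; Sliding door prop that opens and closes in response to switch on and off events.
; Two timelines lerp the door pivot's relative location with sweep, opening to SlidingDirection times DoorHeight and closing to the local origin.
; Each switch event stops the opposite timeline and captures the pivot's current position as the new start, so reversing mid-slide continues from where the door is.
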(event Custom|Stop%20Close
  ;[0.15 0.15 0.15 0.5] Close Door
  (bind _alpha (Timeline|SlideClose Stop)
    (:Update
      (Transformation|SetRelativeLocation (Variables|Default|GetDoorPivot) (Math|Vector|Lerp(Vector) (Variables|Default|GetStarting%20Position) "0, 0, 0" _alpha) true false))))

(event Custom|Stop%20Open
  ;[0.15 0.15 0.15 0.5] Open Door
  (bind _alpha (Timeline|SlideOpen Stop)
    (:Update
      (Transformation|SetRelativeLocation (Variables|Default|GetDoorPivot) (Math|Vector|Lerp(Vector) (Variables|Default|GetStarting%20Position) (Variables|Default|GetFinal%20Position) _alpha) true false))))

(event EventOnSwitchON
  ;[0.15 0.15 0.15 0.5] Open Door
  (CallFunction|StopClose)
  (CallFunction|UpdateStartPosition)
  (CallFunction|UpdateFinalPosition)
  (bind _alpha (Timeline|SlideOpen PlayFromStart)
    (:Update
      (Transformation|SetRelativeLocation (Variables|Default|GetDoorPivot) (Math|Vector|Lerp(Vector) (Variables|Default|GetStarting%20Position) (Variables|Default|GetFinal%20Position) _alpha) true false))))

(event EventOnSwitchOFF
  ;[0.15 0.15 0.15 0.5] Close Door
  (CallFunction|StopOpen)
  (CallFunction|UpdateStartPosition)
  (bind _alpha (Timeline|SlideClose PlayFromStart)
    (:Update
      (Transformation|SetRelativeLocation (Variables|Default|GetDoorPivot) (Math|Vector|Lerp(Vector) (Variables|Default|GetStarting%20Position) "0, 0, 0" _alpha) true false))))

(fn ConstructionScript)

(fn UpdateFinalPosition
  (Variables|Default|SetFinal%20Position (* (Variables|Default|GetSlidingDirection) (Variables|Default|GetDoorHeight))))

(fn UpdateStartPosition
  (Variables|Default|SetStarting%20Position (Variables|/Script/Engine.SceneComponent|GetRelativeLocation (Variables|Default|GetDoorPivot))))