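; Interactable lever prop that animates its handle between off and on angles, then switches its targets.
; The on and off events each play a timeline that lerps the handle pivot's relative rotation.
; Interaction is blocked during the flick; on finish it is re-enabled and SwitchAllTargets is called, so targets change only after the animation completes.
; OnInteract is empty here, and SwitchAllTargets is defined outside this graph.
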(event EventBeginPlay)

(event Collision|EventActorBeginOverlap
  (params (OtherActor :type Actor%20Object%20Reference)))

(event EventTick
  (params (DeltaSeconds :type Float%20%28single-precision%29)))

(event EventOnInteract
  (params (contextActor :type Actor%20Object%20Reference)))

(event EventOnLeveron
  ;[0 0 0 0.5] Update Visual
  (Variables|Default|SetPrevent%20Interaction true)
  (bind _alpha (Timeline|Flick%20On%20Timeline PlayFromStart)
    (:Update
      (Transformation|SetRelativeRotation (Variables|Default|GetHandlePivot) (Math|Rotator|MakeRotator (.X (Math|Vector|BreakVector (Math|Vector|Lerp(Vector) (Variables|Default|GetHandleOFFAngle) (Variables|Default|GetHandleONAngle) _alpha))) (.Y (Math|Vector|BreakVector (Math|Vector|Lerp(Vector) (Variables|Default|GetHandleOFFAngle) (Variables|Default|GetHandleONAngle) _alpha))) (.Z (Math|Vector|BreakVector (Math|Vector|Lerp(Vector) (Variables|Default|GetHandleOFFAngle) (Variables|Default|GetHandleONAngle) _alpha)))) false false))
    (:Finished
      (Variables|Default|SetPrevent%20Interaction false)
      (Class|Lever|SwitchAllTargets))))

(event EventOnLeverOff
  ;[0 0 0 0.5] Update Visual
  (Variables|Default|SetPrevent%20Interaction true)
  (bind _alpha (Timeline|Flick%20Off%20Timeline PlayFromStart)
    (:Update
      (Transformation|SetRelativeRotation (Variables|Default|GetHandlePivot) (Math|Rotator|MakeRotator (.X (Math|Vector|BreakVector (Math|Vector|Lerp(Vector) (Variables|Default|GetHandleONAngle) (Variables|Default|GetHandleOFFAngle) _alpha))) (.Y (Math|Vector|BreakVector (Math|Vector|Lerp(Vector) (Variables|Default|GetHandleONAngle) (Variables|Default|GetHandleOFFAngle) _alpha))) (.Z (Math|Vector|BreakVector (Math|Vector|Lerp(Vector) (Variables|Default|GetHandleONAngle) (Variables|Default|GetHandleOFFAngle) _alpha)))) false false))
    (:Finished
      (Variables|Default|SetPrevent%20Interaction false)
      (Class|Lever|SwitchAllTargets))))

(fn ConstructionScript)

(fn BPCanInteract
  (return (not (Variables|Default|GetPrevent%20Interaction))))