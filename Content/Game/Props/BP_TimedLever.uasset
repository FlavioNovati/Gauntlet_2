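; BP_TimedLever is a lever prop that animates its handle between on and off angles and switches its targets.
; The on and off events each play their own timeline, lerping HandlePivot's relative rotation between HandleOFFAngle and HandleONAngle.
; Each timeline calls SwitchAllTargets when it finishes, so targets change only after the handle completes its swing.
; BPCanInteract always returns false, and no timer logic appears in these graphs.
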(event EventOnLeveron
  ;[0 0 0 0.5] Update Visual
  (bind _alpha (Timeline|Timeline PlayFromStart)
    (:Update
      (Transformation|SetRelativeRotation (Variables|Default|GetHandlePivot) (Math|Rotator|MakeRotator (.X (Math|Vector|BreakVector (Math|Vector|Lerp(Vector) (Variables|Default|GetHandleOFFAngle) (Variables|Default|GetHandleONAngle) _alpha))) (.Y (Math|Vector|BreakVector (Math|Vector|Lerp(Vector) (Variables|Default|GetHandleOFFAngle) (Variables|Default|GetHandleONAngle) _alpha))) (.Z (Math|Vector|BreakVector (Math|Vector|Lerp(Vector) (Variables|Default|GetHandleOFFAngle) (Variables|Default|GetHandleONAngle) _alpha)))) false false))
    (:Finished
      (Class|Lever|SwitchAllTargets))))

(event EventOnLeverOff
  ;[0 0 0 0.5] Update Visual
  (bind _alpha (Timeline|Timeline_0 PlayFromStart)
    (:Update
      (Transformation|SetRelativeRotation (Variables|Default|GetHandlePivot) (Math|Rotator|MakeRotator (.X (Math|Vector|BreakVector (Math|Vector|Lerp(Vector) (Variables|Default|GetHandleONAngle) (Variables|Default|GetHandleOFFAngle) _alpha))) (.Y (Math|Vector|BreakVector (Math|Vector|Lerp(Vector) (Variables|Default|GetHandleONAngle) (Variables|Default|GetHandleOFFAngle) _alpha))) (.Z (Math|Vector|BreakVector (Math|Vector|Lerp(Vector) (Variables|Default|GetHandleONAngle) (Variables|Default|GetHandleOFFAngle) _alpha)))) false false))
    (:Finished
      (Class|Lever|SwitchAllTargets))))

(fn ConstructionScript)

(fn BPCanInteract
  (return false))